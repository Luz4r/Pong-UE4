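; Player-controlled paddle that moves up and down in response to input actions.
; On BeginPlay it passes its Paddle component to SetPaddleReference.
; MovePaddleUp and MovePaddleDown set the component's physics linear velocity along X to positive or negative XSpeed while held.
; Releasing either action zeroes the velocity, even if the other is still held, so movement needs no Tick logic.
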(event `self.ReceiveBeginPlay`
  (`self.SetPaddleReference` (`self.Paddle`)))

(event `InputAction|MovePaddleUp`
  (params (Key :type "Key Structure"))
  (:`Pressed`
    (`PrimitiveComponent.SetPhysicsLinearVelocity` (`self.Paddle`) (`KismetMathLibrary.MakeVector` (`self.XSpeed`)) false "None"))
  (:`Released`
    (`PrimitiveComponent.SetPhysicsLinearVelocity` (`self.Paddle`) (0.0 0.0 0.0) false "None")))

(event `InputAction|MovePaddleDown`
  (params (Key :type "Key Structure"))
  (:`Pressed`
    (`PrimitiveComponent.SetPhysicsLinearVelocity` (`self.Paddle`) (`KismetMathLibrary.MakeVector` (* (`self.XSpeed`) -1.0)) false "None"))
  (:`Released`
    (`PrimitiveComponent.SetPhysicsLinearVelocity` (`self.Paddle`) (0.0 0.0 0.0) false "None")))

(fn `UserConstructionScript`)